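; Tower manager that spawns the tower bases and highlights the tower under the mouse.
; On BeginPlay it spawns a BP_TowerBase slightly above each actor in TowerLocations.
; Each Tick, UpdateHighlight queries GetTowerUnderMouse and compares the result with the cached HighlightedTower.
; Only when they differ does it switch the highlight off on the old tower and on for the new one.
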(event EventBeginPlay
  (for _array_element (Variables|Default|GetTowerLocations)
    (Game|SpawnActorfromClass "/Game/Blueprints/Towers/BP_TowerBase.BP_TowerBase_C" (Math|Transform|MakeTransform (+ (Transformation|GetActorLocation _array_element) "0.000000,0.000000,10.000000") "0, 0, 0" "1.000000,1.000000,1.000000") "Undefined" "MultiplyWithRoot" 0 0)))

(event Collision|EventActorBeginOverlap
  (params (OtherActor :type Actor%20Object%20Reference)))

(event EventTick
  (params (DeltaSeconds :type Float%20%28single-precision%29))
  (CallFunction|UpdateHighlight))

(fn ConstructionScript)

(fn UpdateHighlight
  (Utilities|FlowControl|Sequence
    (:then_0
      (bind (_bisfound _tower) (CallFunction|GetTowerUnderMouse))
      (if _bisfound
        (LocalVariables|SetNewTower _tower)))
    (:then_1
      (if (!= (LocalVariables|GetNewTower) (Variables|Default|GetHighlightedTower))
        (Utilities|FlowControl|Sequence
          (:then_0
            (bind _highlightedtower (Variables|Default|GetHighlightedTower)
              (:then
                (Default|SetHighlight _highlightedtower false))
              (:else)))
          (:then_1
            (bind _output_get (Variables|Default|SetHighlightedTower (LocalVariables|GetNewTower)))
            (Utilities|IsValid _output_get
              (:Is%20Valid
                (Default|SetHighlight _output_get true)))))))))