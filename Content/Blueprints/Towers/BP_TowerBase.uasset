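; BP_TowerBase is a tower actor that supports highlighting and selection.
; SetHighlight toggles the visibility of its Highlight component.
; Select spawns a BP_TowerActions actor slightly above the tower with the tower as owner and stores the reference, which Unselect uses to destroy it.
; The event graph and construction script hold no logic, so all behavior runs through these externally callable functions.
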(event EventBeginPlay)

(event Collision|EventActorBeginOverlap
  (params (OtherActor :type Actor%20Object%20Reference)))

(event EventTick
  (params (DeltaSeconds :type Float%20%28single-precision%29)))

(fn ConstructionScript)

(fn SetHighlight
  (params (bIsHighlighted :type Boolean))
  (Rendering|SetVisibility (Variables|Default|GetHighlight) bIsHighlighted false))

(fn Select
  (bind _returnvalue (Game|SpawnActorfromClass "/Game/UI/BP_TowerActions.BP_TowerActions_C" (Math|Transform|MakeTransform (+ (Transformation|GetActorLocation) "0.000000,0.000000,100.000000") "0, 0, 0" "1.000000,1.000000,1.000000") "Undefined" "MultiplyWithRoot" self 0))
  (Variables|Default|SetBP_TowerActions _returnvalue))

(fn Unselect
  (bind _bp_toweractions (Variables|Default|GetBP_TowerActions)
    (:then
      (Actor|DestroyActor _bp_toweractions)
      (Variables|Default|SetBP_TowerActions 0))
    (:else)))