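; BP_WaveManager is a wave manager that spawns BP_PurpEnemy actors at the start of a Path and moves them along it.
; Each tick, a countdown spawns an enemy at a fixed interval, adds it to the Enemies array and prints the array's size.
; Each enemy advances its own spline distance, which the manager converts to a location.
; Enemies reaching the cached path length are destroyed but never removed from the array.
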(event EventBeginPlay
  (bind _path (Variables|Default|GetPath)
    (:then
      (bind _returnvalue (Default|GetLength _path))
      (Variables|Default|SetPathLength _returnvalue))
    (:else)))

(event Collision|EventActorBeginOverlap
  (params (OtherActor :type Actor%20Object%20Reference)))

(event EventTick
  (params (DeltaSeconds :type Float%20%28single-precision%29))
  (CallFunction|UpdateWave DeltaSeconds))

(fn ConstructionScript)

(fn UpdateWave
  (params (Delta :type Float%20%28double-precision%29))
  (bind _enemies (Variables|Default|GetEnemies))
  (Utilities|FlowControl|Sequence
    (:then_0
      (bind _output_get (Variables|Default|SetTimeUntilEnemy (- (Variables|Default|GetTimeUntilEnemy) Delta)))
      (if (< _output_get 0.0)
        (Variables|Default|SetTimeUntilEnemy 4.0)
        (bind _returnvalue (Default|GetLocation (Variables|Default|GetPath) 0.0))
        (bind _returnvalue_2 (Game|SpawnActorfromClass "/Game/Blueprints/Enemies/BP_PurpEnemy.BP_PurpEnemy_C" (Math|Transform|MakeTransform _returnvalue "0, 0, 0" "1.000000,1.000000,1.000000") "Undefined" "MultiplyWithRoot" 0 0))
        (Utilities|Array|Add _enemies _returnvalue_2)
        (Development|PrintString (Utilities|String|ToString(Integer) (Utilities|Array|Length _enemies)))))
    (:then_1
      (CallFunction|AdvanceEnemies Delta))))

(fn AdvanceEnemies
  (params (Delta :type Float%20%28double-precision%29))
  (for _array_element (Variables|Default|GetEnemies)
    (bind _distance (Default|AdvanceEnemyAlongSpline _array_element Delta))
    (if (< _distance (Variables|Default|GetPathLength))
      (bind _returnvalue (Default|GetLocation (Variables|Default|GetPath) _distance))
      (Transformation|SetActorLocation _array_element _returnvalue false false)
      (else
        (Actor|DestroyActor _array_element)))))