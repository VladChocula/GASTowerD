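; BP_Player is the player Blueprint that handles selecting towers with the mouse.
; A left click calls GetTowerUnderMouse, then selects the found tower or clears the selection when none is hit.
; SelectTower and UnselectTower track a single SelectedTower, notifying it through Select and Unselect and skipping reselection of the same tower.
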(event EventBeginPlay)

(event Collision|EventActorBeginOverlap
  (params (OtherActor :type Actor%20Object%20Reference)))

(event EventTick
  (params (DeltaSeconds :type Float%20%28single-precision%29)))

(event Input|MouseEvents|LeftMouseButton
  (params (Key :type Key%20Structure :default "None"))
  (:Pressed
    (bind (_bisfound _tower) (CallFunction|GetTowerUnderMouse))
    (if _bisfound
      (CallFunction|SelectTower _tower)
      (else
        (CallFunction|UnselectTower)))))

(fn ConstructionScript)

(fn SelectTower
  (params (Tower :type BP%20Tower%20Base%20Object%20Reference))
  (if (!= Tower (Variables|Default|GetSelectedTower))
    (CallFunction|UnselectTower)
    (bind _output_get (Variables|Default|SetSelectedTower Tower))
    (Default|Select _output_get)))

(fn UnselectTower
  (bind _selectedtower (Variables|Default|GetSelectedTower)
    (:then
      (Default|Unselect _selectedtower)
      (Variables|Default|SetSelectedTower 0))
    (:else)))