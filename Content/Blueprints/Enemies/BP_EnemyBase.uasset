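; BP_EnemyBase is a base enemy Blueprint that uses the Gameplay Ability System for its starting attributes and movement along a spline.
; On BeginPlay it applies GE_EnemyAttributes to itself, passing initial health and move speed as SetByCaller magnitudes.
; AdvanceEnemyAlongSpline adds delta times an attribute value to a stored distance and returns it, leaving spline positioning outside this Blueprint.
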(event EventBeginPlay
  (CallFunction|SetInitialEnemyAttributes))

(event Collision|EventActorBeginOverlap
  (params (OtherActor :type Actor%20Object%20Reference)))

(event EventTick
  (params (DeltaSeconds :type Float%20%28single-precision%29)))

(fn ConstructionScript)

(fn SetInitialEnemyAttributes
  (bind _returnvalue (Ability|GameplayEffect|AssignTagSetbyCallerMagnitude (GameplayEffects|MakeOutgoingSpec :self (Variables|Default|GetAbilitySystemComponent) :GameplayEffectClass "/Game/Blueprints/GAS/GameplayEffects/Enemies/GE_EnemyAttributes.GE_EnemyAttributes_C") "(TagName=\"Enemy.Health.SetByCaller\")" (Variables|Default|GetInitialHealth)))
  (bind _returnvalue_2 (Ability|GameplayEffect|AssignTagSetbyCallerMagnitude _returnvalue "(TagName=\"Enemy.MoveSpeed.SetByCaller\")" (Variables|Default|GetInitialMoveSpeed)))
  (GameplayEffects|ApplyGameplayEffectSpecToSelf (Variables|Default|GetAbilitySystemComponent) _returnvalue_2))

(fn AdvanceEnemyAlongSpline
  (params (Delta :type Float%20%28double-precision%29))
  (bind _output_get (Variables|Default|SetDist (+ (* Delta (.ReturnValue (Class|AbilitySystemComponent|GetGameplayAttributeValue (Variables|Default|GetAbilitySystemComponent) "(AttributeName=\"MoveSpeed\",Attribute=/Script/TD1.TD1_EnemyAS:MoveSpeed,AttributeOwner=\"/Script/CoreUObject.Class'/Script/TD1.TD1_EnemyAS'\")"))) (Variables|Default|GetDist))))
  (return _output_get))